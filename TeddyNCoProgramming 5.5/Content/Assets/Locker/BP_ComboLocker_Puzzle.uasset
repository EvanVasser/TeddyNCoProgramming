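; BP_ComboLocker_Puzzle is a three-dial combination locker that opens its door when solved.
; On BeginPlay it registers itself as Parent on three dial child actors.
; CheckSolution stores a dial's position, compares all positions to SolutionParams by building a T/F string, and on "TTT" plays a success sound and rotates the door child actor.
; A DebugMode flag prints positions and results for failed checks.
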(event `self.ReceiveBeginPlay`
  (bind _asbp_locker_combo_1 (cast `/Game/Assets/Locker/SubBlueprints/BP_LockerCombo1` (`ChildActorComponent.ChildActor` (`self.BP_LockerCombo1_C_1`))))
  (set `/Game/Assets/Locker/SubBlueprints/BP_LockerCombo1.Parent` self _asbp_locker_combo_1)
  (bind _asbp_locker_combo_2 (cast `/Game/Assets/Locker/SubBlueprints/BP_LockerCombo2` (`ChildActorComponent.ChildActor` (`self.BP_LockerCombo2_C_1`))))
  (set `/Game/Assets/Locker/SubBlueprints/BP_LockerCombo2.Parent` self _asbp_locker_combo_2)
  (bind _asbp_locker_combo_3 (cast `/Game/Assets/Locker/SubBlueprints/BP_LockerCombo3` (`ChildActorComponent.ChildActor` (`self.BP_LockerCombo3_C_1`))))
  (set `/Game/Assets/Locker/SubBlueprints/BP_LockerCombo3.Parent` self _asbp_locker_combo_3))

(event `Success`
  (`GameplayStatics.PlaySoundAtLocation` "/Game/Assets/Audio/Interaction/Puzzle/Puzzle_Success.Puzzle_Success" (`SceneComponent.K2_GetComponentLocation` (`self.SharedRoot`)) (struct) 1.0 1.0 0.0 null null null null)
  (bind _asbp_locker_door (cast `/Game/Assets/Locker/SubBlueprints/BP_LockerDoor` (`ChildActorComponent.ChildActor` (`self.BP_LockerDoor_C_1`))))
  (`/Game/Assets/Locker/SubBlueprints/BP_LockerDoor.Rotate` _asbp_locker_door))

(event `CheckSolution`
  (params (Position :type Integer) (Combo :type Integer))
  (bind _solution (`self.Solution`))
  (`KismetArrayLibrary.Array_Set` (`self.CurrentPositions`) (- Combo 1) Position)
  (set `self.Solution` "")
  (for (_array_element _array_index) (`self.SolutionParams`)
    (if (== _array_element (`|GetArrayItem` (`self.CurrentPositions`) _array_index))
      (set `self.Solution` (`KismetStringLibrary.Concat_StrStr` _solution "T"))
      (else
        (set `self.Solution` (`KismetStringLibrary.Concat_StrStr` _solution "F")))))
  (if (`KismetStringLibrary.EqualEqual_StrStr` (`self.Solution`) "TTT")
    (`self.Success`)
    (elif (`self.DebugMode`)
      (`self.Debug`))))

(event `ResetCurrentPositions`
  (`KismetArrayLibrary.Array_Clear` (`self.CurrentPositions`))
  (for _ (range 3)
    (`KismetArrayLibrary.Array_Add` (`self.CurrentPositions`))))

(event `Debug`
  (bind _currentpositions (`self.CurrentPositions`))
  (`KismetSystemLibrary.PrintString` (`KismetStringLibrary.Concat_StrStr` (`KismetStringLibrary.Conv_IntToString` (`|GetArrayItem` _currentpositions)) (`KismetStringLibrary.Conv_IntToString` (`|GetArrayItem` _currentpositions 1)) (`KismetStringLibrary.Conv_IntToString` (`|GetArrayItem` _currentpositions 2)) "         " (`self.Solution`)) true true (struct :`G` 0.66 :`B` 1.0 :`A` 1.0) 3.0))

(fn `UserConstructionScript`)
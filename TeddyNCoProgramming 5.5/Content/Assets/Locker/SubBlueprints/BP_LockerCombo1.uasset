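; BP_LockerCombo1 is the first digit dial of a locker combination lock, turned by interaction.
; Each Interact rotates the dial mesh by a 36-degree roll step with MoveComponentTo and plays the lock sound.
; It then advances RotationPosition, wrapping from nine to zero, and passes it with its dial number to the parent's CheckSolution.
; The Inspection function is empty.
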(event `self.Interact`
  (`self.Rotate`)
  (`self.Update Rotation Position`))

(event `Rotate`
  (bind _combolockerdigits_polysurface1 (`self.comboLockerDigits_polySurface1`))
  (bind _returnvalue_roll (`KismetMathLibrary.BreakRotator` (`SceneComponent.K2_GetComponentRotation` _combolockerdigits_polysurface1)))
  (bind _returnvalue_roll_2 (`KismetMathLibrary.BreakRotator` (`KismetMathLibrary.MakeRotator` (+ _returnvalue_roll -36.0))))
  (`KismetSystemLibrary.MoveComponentTo` _combolockerdigits_polysurface1 (0.0 0.0 0.0) (`KismetMathLibrary.MakeRotator` _returnvalue_roll_2))
  (`GameplayStatics.PlaySoundAtLocation` "/Game/Puzzles/lock/combination_lock.combination_lock" (`SceneComponent.RelativeLocation` (`self.comboLockerDigits_polySurface1`)) (struct) 1.0 1.0 0.0 null null null null))

(event `Update Rotation Position`
  (if (> (+ (`self.RotationPosition`) 1) 9)
    (bind _output_get (set `self.RotationPosition` 0))
    (`/Game/Assets/Locker/BP_ComboLocker_Puzzle.CheckSolution` (`self.Parent`) _output_get 1)
    (else
      (bind _output_get_2 (set `self.RotationPosition` (`KismetMathLibrary.Clamp` (+ (`self.RotationPosition`) 1) 0 9)))
      (`/Game/Assets/Locker/BP_ComboLocker_Puzzle.CheckSolution` (`self.Parent`) _output_get_2 1))))

(fn `Inspection`
  (returns (ItemModel :type "StaticMesh Object Reference"))
  (return null))

(fn `UserConstructionScript`)
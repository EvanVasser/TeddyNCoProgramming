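; BP_Spaceship is a spaceship whose pair of doors opens on an Interact event and closes again automatically.
; Each door has an opening and a closing timeline that slide it along local X, with left and right moving in opposite directions.
; A 15-second Delay hanging off each opening Update starts the closing timeline.
; Movement accumulates through AddLocalOffset on every update, so travel distance depends on frame rate.
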(event `self.Interact`
  (`self.OpenLeftDoor`)
  (`self.OpenRightDoor`))

(event `OpenLeftDoor`
  (bind (_direction _leftdoor) (`Timeline|Open`)
    (:`Update`
      (`SceneComponent.K2_AddLocalOffset` (`self.LeftDoor`) (`KismetMathLibrary.MakeVector` (+ 0.0 (* (* _leftdoor -1.0) 1.4))) false false)
      (`KismetSystemLibrary.Delay` 15.0)
      (bind (_direction_2 _leftdoor_2) (`Timeline|Timeline_0`)
        (:`Update`
          (`SceneComponent.K2_AddLocalOffset` (`self.LeftDoor`) (`KismetMathLibrary.MakeVector` (+ 0.0 (* (* _leftdoor_2 1.0) 1.4))) false false))))))

(event `OpenRightDoor`
  (bind (_direction _leftdoor) (`Timeline|Timeline`)
    (:`Update`
      (`SceneComponent.K2_AddLocalOffset` (`self.RightDoor`) (`KismetMathLibrary.MakeVector` (+ 0.0 (* (* _leftdoor 1.0) 1.4))) false false)
      (`KismetSystemLibrary.Delay` 15.0)
      (bind (_direction_2 _leftdoor_2) (`Timeline|Timeline_1`)
        (:`Update`
          (`SceneComponent.K2_AddLocalOffset` (`self.RightDoor`) (`KismetMathLibrary.MakeVector` (+ 0.0 (* (* _leftdoor_2 -1.0) 1.4))) false false))))))

(fn `UserConstructionScript`)
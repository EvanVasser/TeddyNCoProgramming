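; Broad four-panel door in the tutorial level that slides open when its Interact event fires.
; OpenDoors triggers four events at once, each playing its own timeline to slide the left panels (LF, LB) toward local -Y and the right panels (RF, RB) toward +Y.
; Each update adds the scaled curve value as a local offset, so travel accumulates and depends on frame rate.
; There is no closing logic.
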(event `self.Interact`
  (`self.OpenDoors`))

(event `OpenLeftFDoor`
  (bind (_direction _leftdoor) (`Timeline|Timeline`)
    (:`Update`
      (`SceneComponent.K2_AddLocalOffset` (`self.LF`) (`KismetMathLibrary.MakeVector` 0.0 (+ 0.0 (* (* _leftdoor -1.0) 0.8))) false false))))

(event `OpenLeftBDoor`
  (bind (_direction _leftdoor) (`Timeline|Timeline_1`)
    (:`Update`
      (`SceneComponent.K2_AddLocalOffset` (`self.LB`) (`KismetMathLibrary.MakeVector` 0.0 (+ 0.0 (* (* _leftdoor -1.0) 0.8))) false false))))

(event `OpenRightFDoor`
  (bind (_direction _leftdoor) (`Timeline|Timeline_0`)
    (:`Update`
      (`SceneComponent.K2_AddLocalOffset` (`self.RF`) (`KismetMathLibrary.MakeVector` 0.0 (+ 0.0 (* (* _leftdoor 1.0) 0.8))) false false))))

(event `OpenRightBDoor`
  (bind (_direction _leftdoor) (`Timeline|Timeline_2`)
    (:`Update`
      (`SceneComponent.K2_AddLocalOffset` (`self.RB`) (`KismetMathLibrary.MakeVector` 0.0 (+ 0.0 (* (* _leftdoor 1.0) 0.8))) false false))))

(event `OpenDoors`
  (`self.OpenLeftFDoor`)
  (`self.OpenLeftBDoor`)
  (`self.OpenRightFDoor`)
  (`self.OpenRightBDoor`))

(fn `UserConstructionScript`)
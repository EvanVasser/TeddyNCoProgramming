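; BP_DoorTypeNarrow is a narrow double door whose two panels slide in opposite directions on Interact.
; Interact calls OpenDoors, which fires a separate event per panel, each using a FlipFlop to alternate its timeline between Play and Reverse.
; Timeline updates add scaled track values as incremental local Y offsets rather than setting absolute positions.
; F_OpenLeftDoor and F_OpenRightDoor are unused stubs.
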(event `self.Interact`
  (`self.OpenDoors`))

(event `OpenDoors`
  (`self.OpenLeftDoor`)
  (`self.OpenRightDoor`))

(event `OpenLeftDoor`
  (`/Engine/EditorBlueprintResources/StandardMacros.FlipFlop`
    (:`A`
      (bind (_direction _leftdoor) (`Timeline|Timeline` :!label _label)
        (:`Update`
          (`SceneComponent.K2_AddLocalOffset` (`self.LeftDoor`) (`KismetMathLibrary.MakeVector` 0.0 (+ 0.0 (* (* _leftdoor -1.0) 0.6))) false false))
        (:`Finished`)))
    (:`B`
      (goto _label :!via `Reverse`))))

(event `OpenRightDoor`
  (`/Engine/EditorBlueprintResources/StandardMacros.FlipFlop`
    (:`A`
      (bind (_direction _leftdoor) (`Timeline|Timeline_0` :!label _label_2)
        (:`Update`
          (`SceneComponent.K2_AddLocalOffset` (`self.RightDoor`) (`KismetMathLibrary.MakeVector` 0.0 (+ 0.0 (* (* _leftdoor 1.0) 0.6))) false false))
        (:`Finished`)))
    (:`B`
      (goto _label_2 :!via `Reverse`))))

(fn `F_OpenLeftDoor`)

(fn `F_OpenRightDoor`)

(fn `UserConstructionScript`)
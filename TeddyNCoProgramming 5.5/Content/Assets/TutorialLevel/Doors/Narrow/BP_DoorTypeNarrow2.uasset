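; Narrow double-door Blueprint that toggles open and closed on interaction once its HasKey flag is set by PickUPKey.
; InteractITEM calls OpenDoors, which moves both panels and plays a sound, each using a FlipFlop to alternate between opening and closing.
; Separate timelines slide the panels in opposite directions along local Y, adding an offset scaled by DoorConst every update rather than interpolating between fixed positions.
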(event `/Game/Plugs/BPI_interact.InteractITEM`
  (if (`self.HasKey?`)
    (`self.OpenDoors`)))

(event `OpenDoors`
  (`self.OpenLeftDoor`)
  (`self.OpenRightDoor`)
  (`self.PlaySound`))

(event `OpenLeftDoor`
  (`/Engine/EditorBlueprintResources/StandardMacros.FlipFlop`
    (:`A`
      (bind (_direction _leftdoor) (`Timeline|Timeline_1` :!via `PlayFromStart`)
        (:`Update`
          (`SceneComponent.K2_AddLocalOffset` (`self.LeftDoor`) (`KismetMathLibrary.MakeVector` 0.0 (+ 0.0 (* (* _leftdoor -1.0) (`self.DoorConst`)))) false false))))
    (:`B`
      (bind (_direction_2 _leftdoor_2) (`Timeline|Timeline_4` :!via `PlayFromStart`)
        (:`Update`
          (`SceneComponent.K2_AddLocalOffset` (`self.LeftDoor`) (`KismetMathLibrary.MakeVector` 0.0 (+ 0.0 (* (* _leftdoor_2 1.0) (`self.DoorConst`)))) false false))))))

(event `OpenRightDoor`
  (`/Engine/EditorBlueprintResources/StandardMacros.FlipFlop`
    (:`A`
      (bind (_direction _leftdoor) (`Timeline|Timeline_2` :!via `PlayFromStart`)
        (:`Update`
          (`SceneComponent.K2_AddLocalOffset` (`self.RightDoor`) (`KismetMathLibrary.MakeVector` 0.0 (+ 0.0 (* (* _leftdoor 1.0) (`self.DoorConst`)))) false false))))
    (:`B`
      (bind (_direction_2 _leftdoor_2) (`Timeline|Timeline_3` :!via `PlayFromStart`)
        (:`Update`
          (`SceneComponent.K2_AddLocalOffset` (`self.RightDoor`) (`KismetMathLibrary.MakeVector` 0.0 (+ 0.0 (* (* _leftdoor_2 -1.0) (`self.DoorConst`)))) false false))))))

(event `/Game/Plugs/BPI_Door.Pick UP Key`
  (set `self.HasKey?` true))

(event `PlaySound`
  (bind _relativelocation (`SceneComponent.RelativeLocation` (`self.Static_Mesh`)))
  (`/Engine/EditorBlueprintResources/StandardMacros.FlipFlop`
    (:`A`
      (`GameplayStatics.PlaySoundAtLocation` "/Game/Assets/Audio/Interaction/Door_Open.Door_Open" _relativelocation (struct) 1.0 1.0 0.5 null null null null))
    (:`B`
      (`GameplayStatics.PlaySoundAtLocation` "/Game/Assets/Audio/Interaction/Door_Close.Door_Close" _relativelocation (struct) 1.0 1.0 0.5 null null null null))))

(fn `Inspection`
  (returns (ItemModel :type "StaticMesh Object Reference"))
  (return null))

(fn `UserConstructionScript`)
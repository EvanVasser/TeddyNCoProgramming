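; BP_LightObject is a light actor for the tutorial level that combines a SpotLight and a RectLight with configurable start-up state.
; On BeginPlay it optionally applies the Temperature variable to the RectLight only, gated by the SetTemperature flag.
; When IsOn is false it turns both lights off by zeroing their intensity.
; Nothing changes the lights after start-up, and the construction script is empty.
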(event `self.ReceiveBeginPlay`
  (if (`self.setTemperature`)
    (`LightComponent.SetTemperature` (`self.RectLight`) (`self.Temperature`)))
  (if (not (`self.IsOn?`))
    (`LightComponent.SetIntensity` (`self.SpotLight`) 0.0)
    (`LightComponent.SetIntensity` (`self.RectLight`) 0.0)))

(fn `UserConstructionScript`)
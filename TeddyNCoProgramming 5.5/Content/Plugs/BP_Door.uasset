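; BP_Door is a key-locked door that swings open and closed when the player interacts with it.
; PickUPKey sets the Haskey flag, and InteractItem does nothing until that flag is true.
; Each valid interaction alternates through a FlipFlop between playing and reversing DoorTimeline, whose DoorOpen track lerps the static mesh's relative yaw.
; The Inspection function is an empty stub.
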(event `/Game/Plugs/BPI_interact.InteractItem`
  (if (`self.Haskey?`)
    (`/Engine/EditorBlueprintResources/StandardMacros.FlipFlop`
      (:`A`
        (bind (_direction _dooropen) (`Timeline|Door Timeline` :!label _label)
          (:`Update`
            (`SceneComponent.K2_SetRelativeRotation` (`self.StaticMesh`) (`KismetMathLibrary.MakeRotator` 0.0 0.0 (`KismetMathLibrary.Lerp` 0.0 110.0 _dooropen)) false false))))
      (:`B`
        (goto _label :!via `Reverse`)))))

(event `/Game/Plugs/BPI_Door.Pick UP Key`
  (set `self.Haskey?` true))

(fn `Inspection`
  (returns (Itemmodel :type "StaticMesh Object Reference"))
  (return null))

(fn `UserConstructionScript`)
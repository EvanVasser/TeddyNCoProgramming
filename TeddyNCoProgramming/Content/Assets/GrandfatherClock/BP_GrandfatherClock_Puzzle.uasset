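; Grandfather clock puzzle actor that opens two glass doors when its hands are set to the solution positions.
; On BeginPlay it hands itself to the large and small hand child actors as their Parent.
; CheckSolution compares incoming positions with the solution and the other hand's stored position, treating values above 12 as not updated.
; Success plays a song, then after a delay rotates both door child actors.
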(event `self.ReceiveBeginPlay`
  (bind _asbp_gc_large_hand (cast `/Game/Assets/GrandfatherClock/Sub_Blueprints/BP_GC_largeHand` (`ChildActorComponent.ChildActor` (`self.BP_GC_largeHand`))))
  (set `/Game/Assets/GrandfatherClock/Sub_Blueprints/BP_GC_largeHand.Parent` self _asbp_gc_large_hand)
  (bind _asbp_gc_small_hand (cast `/Game/Assets/GrandfatherClock/Sub_Blueprints/BP_GC_smallHand` (`ChildActorComponent.ChildActor` (`self.BP_GC_smallHand`))))
  (set `/Game/Assets/GrandfatherClock/Sub_Blueprints/BP_GC_smallHand.Parent` self _asbp_gc_small_hand))

(event `Check Solution`
  (params (PositionSmall :type Integer :default 13) (PositionLarge :type Integer :default 13))
  (if (== PositionSmall (`self.SolutionParamSmall`))
    (if (== (`self.CurrentPositionLarge`) (`self.SolutionParamLarge`))
      (`self.Success`))
    (elif (== PositionLarge (`self.SolutionParamLarge`))
      (if (== (`self.CurrentPositionSmall`) (`self.SolutionParamSmall`))
        (`self.Success`))))
  (if (> PositionSmall 12)
    (if (not (> PositionLarge 12))
      (set `self.CurrentPositionLarge` PositionLarge))
    (else
      (set `self.CurrentPositionSmall` PositionSmall))))

(event `Success`
  (`KismetSystemLibrary.PrintString` "Success!")
  (`GameplayStatics.PlaySoundAtLocation` "/Game/Assets/Audio/Interaction/Clock/Clock_Song_Success.Clock_Song_Success" (`self.K2_GetActorLocation` self) (struct) 1.0 1.0 0.0 null null null null)
  (`KismetSystemLibrary.Delay` 10.0)
  (bind _asbp_gc_glass_door_1 (cast `/Game/Assets/GrandfatherClock/BP_GC_GlassDoor1` (`ChildActorComponent.ChildActor` (`self.BP_GC_GlassDoor1`))))
  (`/Game/Assets/GrandfatherClock/BP_GC_GlassDoor1.Rotate` _asbp_gc_glass_door_1)
  (bind _asbp_gc_glass_door_2 (cast `/Game/Assets/GrandfatherClock/BP_GC_GlassDoor2` (`ChildActorComponent.ChildActor` (`self.BP_GC_GlassDoor2`))))
  (`/Game/Assets/GrandfatherClock/BP_GC_GlassDoor2.Rotate` _asbp_gc_glass_door_2))

(fn `UserConstructionScript`)
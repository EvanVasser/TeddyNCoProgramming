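; Narrow double sliding door Blueprint in the tutorial level that opens when interacted with.
; Interact calls OpenDoors, which starts separate left and right events, each playing its own timeline.
; Each timeline update adds a scaled local Y offset to its panel, negative for left and positive for right, so movement accumulates per tick.
; The graph contains no closing logic.
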(event `self.Interact`
  (`self.OpenDoors`))

(event `OpenDoors`
  (`self.OpenLeftDoor`)
  (`self.OpenRightDoor`))

(event `OpenLeftDoor`
  (bind (_direction _leftdoor) (`Timeline|Timeline`)
    (:`Update`
      (`SceneComponent.K2_AddLocalOffset` (`self.LeftDoor`) (`KismetMathLibrary.MakeVector` 0.0 (+ 0.0 (* (* _leftdoor -1.0) 0.6))) false false))))

(event `OpenRightDoor`
  (bind (_direction _leftdoor) (`Timeline|Timeline_0`)
    (:`Update`
      (`SceneComponent.K2_AddLocalOffset` (`self.RightDoor`) (`KismetMathLibrary.MakeVector` 0.0 (+ 0.0 (* (* _leftdoor 1.0) 0.6))) false false))))

(fn `UserConstructionScript`)
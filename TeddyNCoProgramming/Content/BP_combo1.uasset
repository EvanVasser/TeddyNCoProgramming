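; BP_combo1 is an interactable mesh that turns when used, apparently one dial of a combination lock.
; Interact prints a debug string, plays the lock sound at the mesh's relative location and eases the mesh to a new pitch.
; The target adds a fixed step to the current world pitch but is applied as relative rotation.
; It tracks no combination value, and the trailing delay leads to nothing.
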(event `self.Interact`
  (bind _static_mesh (`self.Static_Mesh`))
  (bind (_returnvalue_roll _returnvalue_pitch) (`KismetMathLibrary.BreakRotator` (`SceneComponent.K2_GetComponentRotation` _static_mesh)))
  (bind (_returnvalue_roll_2 _returnvalue_pitch_2) (`KismetMathLibrary.BreakRotator` (`KismetMathLibrary.MakeRotator` 0.0 (+ _returnvalue_pitch 40.0))))
  (`KismetSystemLibrary.PrintString` "Hello")
  (`GameplayStatics.PlaySoundAtLocation` "/Game/Puzzles/lock/combination_lock.combination_lock" (`SceneComponent.RelativeLocation` (`self.Static_Mesh`)) (struct) 1.0 1.0 0.0 null null null null)
  (`KismetSystemLibrary.MoveComponentTo` (`self.Static_Mesh`) (`SceneComponent.RelativeLocation` _static_mesh) (`KismetMathLibrary.MakeRotator` 0.0 _returnvalue_pitch_2) true true 0.5)
  (`KismetSystemLibrary.Delay` 0.2))

(fn `UserConstructionScript`)
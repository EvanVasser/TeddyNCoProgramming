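; BP_Button is an interactable button that switches a spot light on and off.
; Its Interatlight event flips the IsLightOn flag and sets the intensity of the referenced Light's spot light component to a fixed lit value or zero.
; Each toggle also prints the new light state as a debug string.
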(event `/Game/Plugs/Interiatbles/BPI_lightinter.Interatlight`
  (bind _spotlightcomponent (`SpotLight.SpotLightComponent` (`self.Light`)))
  (if (not (`self.IsLightOn?`))
    (set `self.IsLightOn?` true)
    (`KismetSystemLibrary.PrintString` "Light On")
    (`LightComponent.SetIntensity` _spotlightcomponent 58.0)
    (else
      (set `self.IsLightOn?` false)
      (`KismetSystemLibrary.PrintString` "Light Off")
      (`LightComponent.SetIntensity` _spotlightcomponent 0.0))))

(fn `UserConstructionScript`)